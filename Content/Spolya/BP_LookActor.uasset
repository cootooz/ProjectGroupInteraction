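; BP_LookActor is a look-at target that registers once when the player's VR camera faces its mesh.
; The construction script applies the MeshSee mesh, and BeginPlay caches the ChildTutorialPawn, hides the mesh and enables its custom depth.
; Once the mesh is unhidden externally, Tick checks only the camera's yaw offset to it, then latches OnSee and disables custom depth when within a narrow angle.
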(event EventBeginPlay
  (bind _aschild_tutorial_pawn (Utilities|Casting|CastToChildTutorialPawn (Game|Player|GetPlayerPawn 0)))
  (Variables|Default|SetPlayer _aschild_tutorial_pawn)
  (Development|SetHiddeninGame (Variables|Default|GetMesh) true false)
  (Rendering|SetRenderCustomDepth (Variables|Default|GetMesh) true))

(event Collision|EventActorBeginOverlap
  (params (OtherActor :type Actor%20Object%20Reference)))

(event EventTick
  (params (DeltaSeconds :type Float%20%28single-precision%29))
  (bind _player (Variables|Default|GetPlayer))
  (bind _cameravr (Variables|/Game/VirtualRealityBP/Blueprints/HandBlueprint/HandControllerPawn.HandControllerPawn_C|GetCameraVR _player))
  (if (not (Variables|Default|GetOnSee?))
    (if (and (< (Math|Float|Absolute(Float) (.Yaw (Math|Rotator|BreakRotator (Math|Rotator|Delta(Rotator) (Math|Rotator|FindLookatRotation (Transformation|GetWorldLocation _cameravr) (Transformation|GetWorldLocation (Variables|Default|GetMesh))) (Transformation|GetWorldRotation _cameravr))))) 1e+01) (not (Variables|/Script/Engine.SceneComponent|GetbHiddenInGame (Variables|Default|GetMesh))))
      (Variables|Default|SetOnSee? true)
      (Rendering|SetRenderCustomDepth (Variables|Default|GetMesh) false))))

(fn ConstructionScript
  (Components|StaticMesh|SetStaticMesh (Variables|Default|GetMesh) (Variables|Default|GetMeshSee)))