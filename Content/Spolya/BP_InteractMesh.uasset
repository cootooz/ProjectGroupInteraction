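; BP_InteractMesh is an actor with a configurable mesh that reacts when a motion controller component overlaps it.
; The construction script assigns MeshInteract to the Mesh component.
; On overlap it turns on custom depth rendering, calls PlayInteract, then turns custom depth off after a short delay.
; PlayInteract checks that the static mesh is valid and switches on InteractType, with no branch behavior connected.
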(event OnComponentBeginOverlap(Mesh)
  (params (OverlappedComponent :type Primitive%20Component%20Object%20Reference) (OtherActor :type Actor%20Object%20Reference) (OtherComp :type Primitive%20Component%20Object%20Reference) (OtherBodyIndex :type Integer) (bFromSweep :type Boolean) (SweepResult :type Hit%20Result%20Structure%20%28by%20ref%29))
  (Utilities|Casting|CastToMotionControllerComponent OtherComp)
  (Rendering|SetRenderCustomDepth (Variables|Default|GetMesh) true)
  (CallFunction|PlayInteract)
  (Utilities|FlowControl|Delay 0.2)
  (Rendering|SetRenderCustomDepth (Variables|Default|GetMesh) false))

(event Custom|PlayInteract
  (Utilities|IsValid (Variables|/Script/Engine.StaticMeshComponent|GetStaticMesh (Variables|Default|GetMesh))
    (:Is%20Valid
      (switch Utilities|FlowControl|Switch|SwitchonInteractType (Variables|Default|GetInteractType)))))

(event EventBeginPlay)

(event Collision|EventActorBeginOverlap
  (params (OtherActor :type Actor%20Object%20Reference)))

(event EventTick
  (params (DeltaSeconds :type Float%20%28single-precision%29)))

(fn ConstructionScript
  (Components|StaticMesh|SetStaticMesh (Variables|Default|GetMesh) (Variables|Default|GetMeshInteract)))